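; Camo_Pig_UnlockBP is an actor that plays a collection animation, apparently for unlocking a camo pig skin.
; Its Harvester event finds the Mini_Game_Pawn and plays a timeline that yaws, uniformly scales and pulls the actor toward the first pawn found.
; Movement lerps from the actor's current location each update, so it follows the pawn's live position without sweeping.
; No unlock logic or destroy step appears in this graph.
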(event Custom|Harvester
  (bind _outactors (Actor|GetAllActorsOfClass "/Game/Blueprints/Blueprints/Mini_Game_Pawn.Mini_Game_Pawn_C"))
  (bind (_direction _rotation _scale _location) (Timeline|Timeline_0 Play)
    (:Update
      (Transformation|SetActorRotation (Math|Rotator|MakeRotator 0.0 0.0 (* _rotation 3.6e+02)))
      (Transformation|SetActorScale3D (Math|Vector|MakeVector _scale _scale _scale))
      (Transformation|SetActorLocation (Math|Vector|Lerp(Vector) (Transformation|GetActorLocation) (Transformation|GetActorLocation (Utilities|Array|Get(acopy) _outactors)) _location) false false))))

(fn ConstructionScript)
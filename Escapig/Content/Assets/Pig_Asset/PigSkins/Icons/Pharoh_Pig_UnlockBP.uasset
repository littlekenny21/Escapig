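; Pharaoh pig skin unlock actor that plays a reveal animation and permanently unlocks the skin.
; Its Harvester event runs a timeline that spins and scales the actor while moving it from a fixed point to just beside the Mini_Game_Pawn.
; When the timeline finishes, it squares the rotation, then sets this skin's slot in the unlocked-skins array to true and saves through SaveGameManager.
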(event Custom|Harvester
  (bind _outactors (Actor|GetAllActorsOfClass "/Game/Blueprints/Blueprints/Mini_Game_Pawn.Mini_Game_Pawn_C"))
  (bind (_direction _rotation _scale _location) (Timeline|Timeline_0 Play)
    (:Update
      (Transformation|SetActorRotation (Math|Rotator|MakeRotator 0.0 0.0 (* _rotation 4.5e+02)))
      (Transformation|SetActorScale3D (Math|Vector|MakeVector _scale _scale _scale))
      (Transformation|SetActorLocation (Math|Vector|Lerp(Vector) "800.000000,250.000000, 0" (Math|Vector|MakeVector (+ (.X (Math|Vector|BreakVector (Transformation|GetActorLocation (Utilities|Array|Get(acopy) _outactors)))) 5e+01) (.Y (Math|Vector|BreakVector (Transformation|GetActorLocation (Utilities|Array|Get(acopy) _outactors)))) (.Z (Math|Vector|BreakVector (Transformation|GetActorLocation (Utilities|Array|Get(acopy) _outactors))))) _location) false false))
    (:Finished
      (Transformation|SetActorRotation "0,90.000000, 0")
      (bind _outactors_2 (Actor|GetAllActorsOfClass "/Game/Blueprints/Blueprints/SaveGameManager.SaveGameManager_C"))
      (Default|LoadUnlockedSkins (Utilities|Array|Get(acopy) _outactors_2))
      (Variables|Default|SetUnlocked%20Skins (Variables|/Game/Blueprints/Blueprints/SaveGameManager.SaveGameManager_C|GetS_UnlockedSkins (Utilities|Array|Get(acopy) _outactors_2)))
      (Utilities|Array|RemoveIndex (Variables|Default|GetUnlocked%20Skins) 16)
      (Utilities|Array|Insert (Variables|Default|GetUnlocked%20Skins) true 16)
      (Default|SaveUnlockedSkins (Utilities|Array|Get(acopy) _outactors_2) (Variables|Default|GetUnlocked%20Skins)))))

(fn ConstructionScript)
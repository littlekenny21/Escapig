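; BP_Cruise is a pickup actor that gives the overlapping PigChar its pickup type through CurrentPickup.
; On sphere overlap, it sets that value, spawns a sound and destroys itself, ignoring components tagged as the truffle magnet trigger.
; A MoveToLocation event lerps it a fraction of the way toward a supplied location on each call, so it can be drawn to the pig.
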(event OnComponentBeginOverlap(Sphere)
  (params (OtherActor :type Actor%20Object%20Reference) (OtherComp :type Primitive%20Component%20Object%20Reference) (OtherBodyIndex :type Integer) (bFromSweep :type Boolean) (SweepResult :type Hit%20Result%20Structure%20%28by%20ref%29))
  (bind _aspig_char (Utilities|Casting|CastToPigChar OtherActor))
  (if (not (Components|ComponentHasTag OtherComp "truffleTrigger(magnet)"))
    (Variables|/Game/Blueprints/Blueprints/PigChar.PigChar_C|SetCurrent_Pickup _aspig_char 4)
    (Audio|SpawnSoundatLocation 0 (Transformation|GetActorLocation))
    (Actor|DestroyActor)))

(event Custom|MoveToLocation
  (params (Location :type Vector))
  ;[1 1 1] linearly interpolates towards the given location which will be the pig
  (Transformation|SetActorLocation (Math|Vector|Lerp(Vector) Location (Transformation|GetActorLocation) 0.85) false false))

(fn ConstructionScript)
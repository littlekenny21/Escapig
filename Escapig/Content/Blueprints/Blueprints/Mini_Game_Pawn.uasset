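; Mini-game pawn that sets up the on-screen UI for the harvester mini-game or the customisation mode, chosen by boolean flags.
; On BeginPlay, harvester mode shows its mini-game widget, while plot mode adds nothing.
; Customise mode waits briefly, loads unlocked skins from the SaveGameManager actor, then opens and begins the Customise widget.
; Possession clears all existing widgets.
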(event EventBeginPlay
  (if (Variables|Default|GetHarvester_Mini_Game)
    (bind _returnvalue (UserInterface|CreateWidget "/Game/UMG/Harvester_Mini_Game_UI.Harvester_Mini_Game_UI_C"))
    (UserInterface|Viewport|AddtoViewport _returnvalue 0)
    (elif (not (Variables|Default|GetPlot_Mini_Game))
      (if (Variables|Default|GetCustomise)
        (Utilities|FlowControl|Delay 0.1)
        (bind _outactors (Actor|GetAllActorsOfClass "/Game/Blueprints/Blueprints/SaveGameManager.SaveGameManager_C"))
        (Default|LoadUnlockedSkins (Utilities|Array|Get(acopy) _outactors))
        (Variables|Default|SetUnlocked%20Skins (Variables|/Game/Blueprints/Blueprints/SaveGameManager.SaveGameManager_C|GetS_UnlockedSkins (Utilities|Array|Get(acopy) _outactors)))
        (bind _returnvalue_2 (UserInterface|CreateWidget "/Game/UMG/Customise.Customise_C"))
        (UserInterface|Viewport|AddtoViewport _returnvalue_2 0)
        (Default|Begin _returnvalue_2)))))

(event EventPossessed
  (params (NewController :type Controller%20Object%20Reference))
  (Viewport|RemoveAllWidgets))

(fn ConstructionScript)
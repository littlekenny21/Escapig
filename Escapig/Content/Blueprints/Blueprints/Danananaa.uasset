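; Actor that shows a randomly chosen loading-style backdrop behind an animated sprite.
; On BeginPlay it applies one of six Load_Back materials to the Cube, then starts an endless Delay-driven loop.
; Each pass rotates the PaperSprite and sets its scale from NoseScale, which grows and shrinks between limits as the Updown flag flips, giving a spinning, pulsing effect.
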(event EventBeginPlay
  (bind _papersprite (Variables|Default|GetPaperSprite))
  (switch int (Math|Random|RandomIntegerinRange 0 5)
    (:0
      (Rendering|Material|SetMaterial (Variables|Default|GetCube) 0 "/Game/Assets/LoadBacking/Load_Back_Mat.Load_Back_Mat"))
    (:1
      (Rendering|Material|SetMaterial (Variables|Default|GetCube) 0 "/Game/Assets/LoadBacking/Load_Back1_Mat.Load_Back1_Mat"))
    (:2
      (Rendering|Material|SetMaterial (Variables|Default|GetCube) 0 "/Game/Assets/LoadBacking/Load_Back2_Mat.Load_Back2_Mat"))
    (:3
      (Rendering|Material|SetMaterial (Variables|Default|GetCube) 0 "/Game/Assets/LoadBacking/Load_Back3_Mat.Load_Back3_Mat"))
    (:4
      (Rendering|Material|SetMaterial (Variables|Default|GetCube) 0 "/Game/Assets/LoadBacking/Load_Back4_Mat.Load_Back4_Mat"))
    (:5
      (Rendering|Material|SetMaterial (Variables|Default|GetCube) 0 "/Game/Assets/LoadBacking/Load_Back5_Mat.Load_Back5_Mat")))
  (Transformation|AddLocalRotation _papersprite "2.000000, 0, 0" false false :!label _label)
  (Transformation|SetRelativeScale3D _papersprite (Variables|Default|GetNose_Scale))
  (switch int (Variables|Default|Getup/down)
    (:0
      (if (Math|Vector|Equal(Vector) (Variables|Default|GetNose_Scale) "5.000000, 0,5.000000" 0.5)
        (Variables|Default|Setup/down 1))
      (Utilities|FlowControl|Delay 0.01)
      (Variables|Default|SetNose_Scale (+ (Variables|Default|GetNose_Scale) "0.100000,0.000000,0.100000"))
      (goto _label))
    (:1
      (if (Math|Vector|Equal(Vector) (Variables|Default|GetNose_Scale) "0.200000,0.000000,0.200000" 0.5)
        (Variables|Default|Setup/down 0))
      (Utilities|FlowControl|Delay 0.01)
      (Variables|Default|SetNose_Scale (- (Variables|Default|GetNose_Scale) "0.100000, 0,0.100000"))
      (goto _label))))

(fn ConstructionScript)
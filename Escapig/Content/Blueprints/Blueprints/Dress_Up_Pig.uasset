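; Dress-up pig Blueprint that shows an animated pig character with a swappable skin texture.
; On BeginPlay, PigChar loops a trot animation and gets a dynamic instance of the pig material, whose "Skin" texture is cached in the Skin variable.
; The Skin_Change event writes the current Skin variable back into that material parameter, so a new texture assigned to the variable appears on the pig.
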(event Custom|Skin_Change
  (Rendering|Material|SetTextureParameterValue (Variables|Default|GetDress) "Skin" (Variables|Default|GetSkin)))

(event EventBeginPlay
  (Components|Animation|PlayAnimation (Variables|Default|GetPig_Char) "/Game/Assets/Pig_Asset/Pig_anims/pig_trott.pig_trott" true)
  (bind _returnvalue (Rendering|Material|CreateDynamicMaterialInstance (Variables|Default|GetPig_Char) 0 "/Game/Assets/Pig_Asset/Pig_mat.Pig_mat" :!class /Script/Engine.PrimitiveComponent))
  (bind _output_get (Variables|Default|SetDress _returnvalue))
  (bind _returnvalue_2 (Rendering|Material|GetTextureParameterValue _output_get "Skin" :!class /Script/Engine.MaterialInstanceDynamic))
  (Variables|Default|SetSkin _returnvalue_2))

(fn ConstructionScript)
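; A plot actor whose grid of static meshes is cleared row by row by a spawned Harvester when clicked or touched.
; On BeginPlay it sorts its mesh components into seven row arrays.
; A click or touch spawns a Harvester just offset from the plot, flagged for minigame mode with mincing off, then hides each row in turn on short delays for a progressive harvest effect.
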(event MouseInput|EventActorOnClicked
  (bind _returnvalue (Transformation|GetActorLocation))
  (bind (_x _y _z) (Math|Vector|BreakVector _returnvalue))
  (bind _returnvalue_2 (Game|SpawnActorfromClass "/Game/Blueprints/Blueprints/Harvester.Harvester_C" (Math|Transform|MakeTransform (Math|Vector|MakeVector (- _x 5e+01) _y _z) (Transformation|GetActorRotation)) "Undefined" 0 0))
  (Variables|/Game/Blueprints/Blueprints/Harvester.Harvester_C|SetMini_Game _returnvalue_2 true)
  (Variables|/Game/Blueprints/Blueprints/Harvester.Harvester_C|SetMince _returnvalue_2 false)
  (Utilities|FlowControl|Delay 0.1)
  (for _array_element (Variables|Default|Getrow%201)
    (Rendering|SetVisibility _array_element false false))
  (Utilities|FlowControl|Delay 0.1)
  (for _array_element_2 (Variables|Default|Getrow%202)
    (Rendering|SetVisibility _array_element_2 false false))
  (Utilities|FlowControl|Delay 0.1)
  (for _array_element_3 (Variables|Default|Getrow%203)
    (Rendering|SetVisibility _array_element_3 false false))
  (Utilities|FlowControl|Delay 0.1)
  (for _array_element_4 (Variables|Default|Getrow%204)
    (Rendering|SetVisibility _array_element_4 false false))
  (Utilities|FlowControl|Delay 0.1)
  (for _array_element_5 (Variables|Default|Getrow%205)
    (Rendering|SetVisibility _array_element_5 false false))
  (Utilities|FlowControl|Delay 0.1)
  (for _array_element_6 (Variables|Default|Getrow%206)
    (Rendering|SetVisibility _array_element_6 false false))
  (Utilities|FlowControl|Delay 0.1)
  (for _array_element_7 (Variables|Default|Getrow%207)
    (Rendering|SetVisibility _array_element_7 false false)))

(event EventActorOnInputTouchBegin
  (params (FingerIndex :type ETouchIndex%20Enum :default "Touch1"))
  (bind _returnvalue (Transformation|GetActorLocation))
  (bind (_x _y _z) (Math|Vector|BreakVector _returnvalue))
  (bind _returnvalue_2 (Game|SpawnActorfromClass "/Game/Blueprints/Blueprints/Harvester.Harvester_C" (Math|Transform|MakeTransform (Math|Vector|MakeVector (- _x 5e+01) _y _z) (Transformation|GetActorRotation)) "Undefined" 0 0))
  (Variables|/Game/Blueprints/Blueprints/Harvester.Harvester_C|SetMini_Game _returnvalue_2 true)
  (Variables|/Game/Blueprints/Blueprints/Harvester.Harvester_C|SetMince _returnvalue_2 false)
  (Utilities|FlowControl|Delay 0.1)
  (for _array_element (Variables|Default|Getrow%201)
    (Rendering|SetVisibility _array_element false false))
  (Utilities|FlowControl|Delay 0.1)
  (for _array_element_2 (Variables|Default|Getrow%202)
    (Rendering|SetVisibility _array_element_2 false false))
  (Utilities|FlowControl|Delay 0.1)
  (for _array_element_3 (Variables|Default|Getrow%203)
    (Rendering|SetVisibility _array_element_3 false false))
  (Utilities|FlowControl|Delay 0.1)
  (for _array_element_4 (Variables|Default|Getrow%204)
    (Rendering|SetVisibility _array_element_4 false false))
  (Utilities|FlowControl|Delay 0.1)
  (for _array_element_5 (Variables|Default|Getrow%205)
    (Rendering|SetVisibility _array_element_5 false false))
  (Utilities|FlowControl|Delay 0.1)
  (for _array_element_6 (Variables|Default|Getrow%206)
    (Rendering|SetVisibility _array_element_6 false false))
  (Utilities|FlowControl|Delay 0.1)
  (for _array_element_7 (Variables|Default|Getrow%207)
    (Rendering|SetVisibility _array_element_7 false false)))

(event EventBeginPlay
  (bind _row_7 (Variables|Default|Getrow%207))
  (bind _row_1 (Variables|Default|Getrow%201))
  (bind _row_2 (Variables|Default|Getrow%202))
  (bind _row_3 (Variables|Default|Getrow%203))
  (bind _row_4 (Variables|Default|Getrow%204))
  (bind _row_5 (Variables|Default|Getrow%205))
  (bind _row_6 (Variables|Default|Getrow%206))
  (Utilities|Array|Add _row_1 (Variables|Default|GetStaticMesh5))
  (Utilities|Array|Add _row_1 (Variables|Default|GetStaticMesh11))
  (Utilities|Array|Add _row_1 (Variables|Default|GetStaticMesh17))
  (Utilities|Array|Add _row_1 (Variables|Default|GetStaticMesh24))
  (Utilities|Array|Add _row_1 (Variables|Default|GetStaticMesh31))
  (Utilities|Array|Add _row_1 (Variables|Default|GetStaticMesh39))
  (Utilities|Array|Add _row_1 (Variables|Default|GetStaticMesh46))
  (Utilities|Array|Add _row_2 (Variables|Default|GetStaticMesh4))
  (Utilities|Array|Add _row_2 (Variables|Default|GetStaticMesh10))
  (Utilities|Array|Add _row_2 (Variables|Default|GetStaticMesh16))
  (Utilities|Array|Add _row_2 (Variables|Default|GetStaticMesh23))
  (Utilities|Array|Add _row_2 (Variables|Default|GetStaticMesh30))
  (Utilities|Array|Add _row_2 (Variables|Default|GetStaticMesh38))
  (Utilities|Array|Add _row_2 (Variables|Default|GetStaticMesh45))
  (Utilities|Array|Add _row_3 (Variables|Default|GetStaticMesh1))
  (Utilities|Array|Add _row_3 (Variables|Default|GetStaticMesh7))
  (Utilities|Array|Add _row_3 (Variables|Default|GetStaticMesh20))
  (Utilities|Array|Add _row_3 (Variables|Default|GetStaticMesh27))
  (Utilities|Array|Add _row_3 (Variables|Default|GetStaticMesh34))
  (Utilities|Array|Add _row_3 (Variables|Default|GetStaticMesh35))
  (Utilities|Array|Add _row_3 (Variables|Default|GetStaticMesh42))
  (Utilities|Array|Add _row_4 (Variables|Default|GetStaticMesh))
  (Utilities|Array|Add _row_4 (Variables|Default|GetStaticMesh13))
  (Utilities|Array|Add _row_4 (Variables|Default|GetStaticMesh19))
  (Utilities|Array|Add _row_4 (Variables|Default|GetStaticMesh26))
  (Utilities|Array|Add _row_4 (Variables|Default|GetStaticMesh33))
  (Utilities|Array|Add _row_4 (Variables|Default|GetStaticMesh41))
  (Utilities|Array|Add _row_4 (Variables|Default|GetStaticMesh48))
  (Utilities|Array|Add _row_5 (Variables|Default|GetStaticMesh2))
  (Utilities|Array|Add _row_5 (Variables|Default|GetStaticMesh8))
  (Utilities|Array|Add _row_5 (Variables|Default|GetStaticMesh14))
  (Utilities|Array|Add _row_5 (Variables|Default|GetStaticMesh21))
  (Utilities|Array|Add _row_5 (Variables|Default|GetStaticMesh28))
  (Utilities|Array|Add _row_5 (Variables|Default|GetStaticMesh36))
  (Utilities|Array|Add _row_5 (Variables|Default|GetStaticMesh43))
  (Utilities|Array|Add _row_6 (Variables|Default|GetStaticMesh3))
  (Utilities|Array|Add _row_6 (Variables|Default|GetStaticMesh9))
  (Utilities|Array|Add _row_6 (Variables|Default|GetStaticMesh15))
  (Utilities|Array|Add _row_6 (Variables|Default|GetStaticMesh22))
  (Utilities|Array|Add _row_6 (Variables|Default|GetStaticMesh29))
  (Utilities|Array|Add _row_6 (Variables|Default|GetStaticMesh37))
  (Utilities|Array|Add _row_6 (Variables|Default|GetStaticMesh44))
  (Utilities|Array|Add _row_7 (Variables|Default|GetStaticMesh6))
  (Utilities|Array|Add _row_7 (Variables|Default|GetStaticMesh12))
  (Utilities|Array|Add _row_7 (Variables|Default|GetStaticMesh18))
  (Utilities|Array|Add _row_7 (Variables|Default|GetStaticMesh25))
  (Utilities|Array|Add _row_7 (Variables|Default|GetStaticMesh32))
  (Utilities|Array|Add _row_7 (Variables|Default|GetStaticMesh40))
  (Utilities|Array|Add _row_7 (Variables|Default|GetStaticMesh47)))

(fn ConstructionScript)
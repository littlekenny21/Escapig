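; Endless-runner floor tile for the pig character, which requests the next tile from Escapig_Mode at its end trigger, then destroys itself after a delay.
; Construction script spawns a blocker, truffle or power-up through chained weight checks, each re-rolling its random number.
; Blocker odds and chances of a second blocker rise with distance travelled; low CurrentStraits substitutes a truffle.
; Wall hits cost a life when the normal aligns with the pig's forward vector.
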(event OnComponentBeginOverlap(End_Trigger)
  (params (OtherActor :type Actor%20Object%20Reference) (OtherComp :type Primitive%20Component%20Object%20Reference) (OtherBodyIndex :type Integer) (bFromSweep :type Boolean) (SweepResult :type Hit%20Result%20Structure%20%28by%20ref%29))
  (Utilities|Casting|CastToPigChar OtherActor)
  (bind _asescapig_mode (Utilities|Casting|CastToEscapig_Mode (Game|GetGameMode)))
  (Utilities|FlowControl|Sequence
    (:then_0
      (Utilities|FlowControl|DoOnce false
        (:Completed
          (Default|AddFloorTile _asescapig_mode))))
    (:then_1
      (Utilities|FlowControl|Delay 5.0)
      (Actor|DestroyActor))))

(event OnComponentHit(wall)
  (params (OtherActor :type Actor%20Object%20Reference) (OtherComp :type Primitive%20Component%20Object%20Reference) (NormalImpulse :type Vector :default "0, 0, 0") (Hit :type Hit%20Result%20Structure%20%28by%20ref%29))
  ;[1 1 1] wall collisons
  (bind _aspig_char (Utilities|Casting|CastToPigChar OtherActor))
  (if (Math|Float|NearlyEqual(Float) (Math|Vector|DotProduct (.normal Hit) (Transformation|GetActorForwardVector _aspig_char)) 1.0 0.01)
    (Default|LifeLost _aspig_char)))

(event OnComponentHit(wall2)
  (params (OtherActor :type Actor%20Object%20Reference) (OtherComp :type Primitive%20Component%20Object%20Reference) (NormalImpulse :type Vector :default "0, 0, 0") (Hit :type Hit%20Result%20Structure%20%28by%20ref%29))
  ;[1 1 1] wall collisons
  (bind _aspig_char (Utilities|Casting|CastToPigChar OtherActor))
  (if (Math|Float|NearlyEqual(Float) (Math|Vector|DotProduct (.normal Hit) (Transformation|GetActorForwardVector _aspig_char)) 1.0 0.01)
    (Default|LifeLost _aspig_char)))

(event EventBeginPlay)

(event Collision|EventActorBeginOverlap
  (params (OtherActor :type Actor%20Object%20Reference)))

(event EventTick
  (params (DeltaSeconds :type Float%20%28single-precision%29)))

(fn ConstructionScript
  (CallFunction|RandomiseTexture)
  (CallFunction|SetSpawnPoints)
  (bind _outactors (Actor|GetAllActorsOfClass "/Game/Blueprints/Blueprints/PigChar.PigChar_C"))
  (Variables|Default|SetBlockerProbability (+ (Variables|Default|GetBlockerProbability) (Math|Float|Truncate (/ (Variables|/Game/Blueprints/Blueprints/PigChar.PigChar_C|GetTotalDistance (Utilities|Array|Get(acopy) _outactors)) 1e+06))))
  (Variables|Default|SetMaxProbabilityNum (+ (+ (+ (+ (+ (+ (Variables|Default|GetBlockerProbability) (Variables|Default|GetTruffleProbability)) (Variables|Default|GetExtraLifeProbability)) (Variables|Default|GetMagnetProbability)) (Variables|Default|GetCruiseProbability)) (Variables|Default|GetSlowHarvesterProbability)) (Variables|Default|GetBoarChargeProbability)))
  (if (> (Math|Random|RandomIntegerinRange 0 (Variables|Default|GetMaxProbabilityNum)) 0)
    (if (<= (Math|Random|RandomIntegerinRange 0 (Variables|Default|GetMaxProbabilityNum)) (Variables|Default|GetBlockerProbability))
      (bind _asescapig_mode (Utilities|Casting|CastToEscapig_Mode (Game|GetGameMode) :!label _label))
      (if (<= (Variables|/Game/Blueprints/Blueprints/Escapig_Mode.Escapig_Mode_C|GetCurrent_Straits _asescapig_mode) 1)
        (CallFunction|SpawnTruffle)
        (else
          (CallFunction|SpawnBlocker)))
      (else
        (if (> (Math|Random|RandomIntegerinRange 0 (Variables|Default|GetMaxProbabilityNum)) (Variables|Default|GetBlockerProbability)) :!label _label_2
          (if (<= (Math|Random|RandomIntegerinRange 0 (Variables|Default|GetMaxProbabilityNum)) (+ (Variables|Default|GetBlockerProbability) (Variables|Default|GetTruffleProbability)))
            (CallFunction|SpawnTruffle)
            (else
              (if (> (Math|Random|RandomIntegerinRange 0 (Variables|Default|GetMaxProbabilityNum)) (+ (Variables|Default|GetBlockerProbability) (Variables|Default|GetTruffleProbability))) :!label _label_3
                (if (<= (Math|Random|RandomIntegerinRange 0 (Variables|Default|GetMaxProbabilityNum)) (+ (+ (Variables|Default|GetBlockerProbability) (Variables|Default|GetTruffleProbability)) (Variables|Default|GetExtraLifeProbability)))
                  (CallFunction|SpawnExtraLife)
                  (else
                    (if (> (Math|Random|RandomIntegerinRange 0 (Variables|Default|GetMaxProbabilityNum)) (+ (+ (Variables|Default|GetBlockerProbability) (Variables|Default|GetTruffleProbability)) (Variables|Default|GetExtraLifeProbability))) :!label _label_4
                      (if (<= (Math|Random|RandomIntegerinRange 0 (Variables|Default|GetMaxProbabilityNum)) (+ (+ (+ (Variables|Default|GetBlockerProbability) (Variables|Default|GetTruffleProbability)) (Variables|Default|GetExtraLifeProbability)) (Variables|Default|GetMagnetProbability)))
                        (CallFunction|SpawnMagnet)
                        (else
                          (if (> (Math|Random|RandomIntegerinRange 0 (Variables|Default|GetMaxProbabilityNum)) (+ (+ (+ (Variables|Default|GetBlockerProbability) (Variables|Default|GetTruffleProbability)) (Variables|Default|GetExtraLifeProbability)) (Variables|Default|GetMagnetProbability))) :!label _label_5
                            (if (<= (Math|Random|RandomIntegerinRange 0 (Variables|Default|GetMaxProbabilityNum)) (+ (+ (+ (+ (Variables|Default|GetBlockerProbability) (Variables|Default|GetTruffleProbability)) (Variables|Default|GetExtraLifeProbability)) (Variables|Default|GetMagnetProbability)) (Variables|Default|GetCruiseProbability)))
                              (CallFunction|SpawnCruise)
                              (else
                                (if (> (Math|Random|RandomIntegerinRange 0 (Variables|Default|GetMaxProbabilityNum)) (+ (+ (+ (+ (Variables|Default|GetBlockerProbability) (Variables|Default|GetTruffleProbability)) (Variables|Default|GetExtraLifeProbability)) (Variables|Default|GetMagnetProbability)) (Variables|Default|GetCruiseProbability))) :!label _label_6
                                  (if (<= (Math|Random|RandomIntegerinRange 0 (Variables|Default|GetMaxProbabilityNum)) (+ (+ (+ (+ (+ (Variables|Default|GetBlockerProbability) (Variables|Default|GetTruffleProbability)) (Variables|Default|GetExtraLifeProbability)) (Variables|Default|GetMagnetProbability)) (Variables|Default|GetCruiseProbability)) (Variables|Default|GetSlowHarvesterProbability)))
                                    (CallFunction|SpawnSlowHarvester)
                                    (else
                                      (if (> (Math|Random|RandomIntegerinRange 0 (Variables|Default|GetMaxProbabilityNum)) (+ (+ (+ (+ (+ (Variables|Default|GetBlockerProbability) (Variables|Default|GetTruffleProbability)) (Variables|Default|GetExtraLifeProbability)) (Variables|Default|GetMagnetProbability)) (Variables|Default|GetCruiseProbability)) (Variables|Default|GetSlowHarvesterProbability))) :!label _label_7
                                        (if (<= (Math|Random|RandomIntegerinRange 0 (Variables|Default|GetMaxProbabilityNum)) (+ (+ (+ (+ (+ (+ (Variables|Default|GetBlockerProbability) (Variables|Default|GetTruffleProbability)) (Variables|Default|GetExtraLifeProbability)) (Variables|Default|GetMagnetProbability)) (Variables|Default|GetCruiseProbability)) (Variables|Default|GetSlowHarvesterProbability)) (Variables|Default|GetBoarChargeProbability)))
                                          (CallFunction|SpawnBoarCharge)
                                          (else
                                            (goto _label)))
                                        (else
                                          (goto _label)))))
                                  (else
                                    (goto _label_7)))))
                            (else
                              (goto _label_6)))))
                      (else
                        (goto _label_5)))))
                (else
                  (goto _label_4)))))
          (else
            (goto _label_3)))))
    (else
      (goto _label_2))))

(fn GetAttachTransform
  (return (Transformation|GetWorldTransform (Variables|Default|GetAttach_Point))))

(fn SetSpawnPoints
  (Variables|Default|SetSpawnPoints (Utilities|Array|MakeArray (Transformation|GetRelativeTransform (Variables|Default|GetSpawnpoint)) (Transformation|GetRelativeTransform (Variables|Default|GetSpawnpointR)) (Transformation|GetRelativeTransform (Variables|Default|GetSpawnPointL)))))

(fn SpawnBlocker
  (bind _returnvalue (Math|Random|RandomIntegerinRange 0 0))
  (bind _spawnpoints (Variables|Default|GetSpawnPoints))
  (bind _output_get (Variables|Default|SetBlockerSpawnedLocation (Math|Random|RandomIntegerinRange 0 (Utilities|Array|LastIndex _spawnpoints))))
  (switch int (Math|Random|RandomIntegerinRange 0 0)
    (:0
      (AddComponent|AddChildActorComponent false (Utilities|Array|Get(acopy) _spawnpoints _output_get))
      (bind _outactors (Actor|GetAllActorsOfClass "/Game/Blueprints/Blueprints/PigChar.PigChar_C"))
      (if (>= (Math|Float|Truncate (/ (Variables|/Game/Blueprints/Blueprints/PigChar.PigChar_C|GetTotalDistance (Utilities|Array|Get(acopy) _outactors)) 1e+04)) 200)
        (if (>= (Math|Float|Truncate (/ (Variables|/Game/Blueprints/Blueprints/PigChar.PigChar_C|GetTotalDistance (Utilities|Array|Get(acopy) _outactors)) 1e+04)) 600)
          (Variables|Default|SetTempBlockerLocation 0 :!label _label)
          (if (== (Variables|Default|GetTempBlockerLocation) (Variables|Default|GetBlockerSpawnedLocation))
            (Variables|Default|SetTempBlockerLocation 0)
            (if (not (== (Variables|Default|GetTempBlockerLocation) (Variables|Default|GetBlockerSpawnedLocation)))
              (switch int _returnvalue
                (:0
                  (AddComponent|AddChildActorComponent false (Utilities|Array|Get(acopy) (Variables|Default|GetSpawnPoints) (Variables|Default|GetTempBlockerLocation))))))
            (else
              (switch int _returnvalue
                (:0
                  (AddComponent|AddChildActorComponent false (Utilities|Array|Get(acopy) (Variables|Default|GetSpawnPoints) (Variables|Default|GetTempBlockerLocation)))))))
          (elif (== (Math|Random|RandomIntegerinRange 0 1) 1)
            (goto _label)))))))

(fn SpawnTruffle
  (bind _truffel_area (Variables|Default|GetTruffel%20Area))
  (for _index (range 0 0)
    (AddComponent|AddChildActorComponent false (Math|Conversions|ToTransform(Vector) (Math|Random|RandomPointinBoundingBox (Variables|/Script/Engine.SceneComponent|GetRelativeLocation _truffel_area) (Variables|/Script/Engine.BoxComponent|GetBoxExtent _truffel_area))))))

(fn GetMidPoint
  (return (Transformation|GetWorldLocation (Variables|Default|GetMidPoint))))

(fn SpawnExtraLife
  (bind _truffel_area (Variables|Default|GetTruffel%20Area))
  (for _index (range 0 0)
    (AddComponent|AddChildActorComponent false (Math|Conversions|ToTransform(Vector) (Math|Random|RandomPointinBoundingBox (Variables|/Script/Engine.SceneComponent|GetRelativeLocation _truffel_area) (Variables|/Script/Engine.BoxComponent|GetBoxExtent _truffel_area))))))

(fn SpawnBoarCharge
  (bind _truffel_area (Variables|Default|GetTruffel%20Area))
  (for _index (range 0 0)
    (AddComponent|AddChildActorComponent false (Math|Conversions|ToTransform(Vector) (Math|Random|RandomPointinBoundingBox (Variables|/Script/Engine.SceneComponent|GetRelativeLocation _truffel_area) (Variables|/Script/Engine.BoxComponent|GetBoxExtent _truffel_area))))))

(fn SpawnMagnet
  (bind _truffel_area (Variables|Default|GetTruffel%20Area))
  (for _index (range 0 0)
    (AddComponent|AddChildActorComponent false (Math|Conversions|ToTransform(Vector) (Math|Random|RandomPointinBoundingBox (Variables|/Script/Engine.SceneComponent|GetRelativeLocation _truffel_area) (Variables|/Script/Engine.BoxComponent|GetBoxExtent _truffel_area))))))

(fn SpawnSlowHarvester
  (bind _truffel_area (Variables|Default|GetTruffel%20Area))
  (for _index (range 0 0)
    (AddComponent|AddChildActorComponent false (Math|Conversions|ToTransform(Vector) (Math|Random|RandomPointinBoundingBox (Variables|/Script/Engine.SceneComponent|GetRelativeLocation _truffel_area) (Variables|/Script/Engine.BoxComponent|GetBoxExtent _truffel_area))))))

(fn SpawnCruise
  (bind _truffel_area (Variables|Default|GetTruffel%20Area))
  (for _index (range 0 0)
    (AddComponent|AddChildActorComponent false (Math|Conversions|ToTransform(Vector) (Math|Random|RandomPointinBoundingBox (Variables|/Script/Engine.SceneComponent|GetRelativeLocation _truffel_area) (Variables|/Script/Engine.BoxComponent|GetBoxExtent _truffel_area))))))

(fn RandomiseTexture)
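; Tree obstacle Blueprint that blocks the pig character and varies its appearance.
; The Construction Script calls RandomiseSize, scaling the Cube uniformly within a min/max range and randomly applying one of two tree materials.
; When PigChar hits the Cube, a charging pig destroys the tree, while a non-charging pig loses a life.
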(event OnComponentHit(Cube)
  (params (OtherActor :type Actor%20Object%20Reference) (OtherComp :type Primitive%20Component%20Object%20Reference) (NormalImpulse :type Vector :default "0, 0, 0") (Hit :type Hit%20Result%20Structure%20%28by%20ref%29))
  (bind _aspig_char (Utilities|Casting|CastToPigChar OtherActor))
  (if (Variables|/Game/Blueprints/Blueprints/PigChar.PigChar_C|GetCHARGE! _aspig_char)
    (Actor|DestroyActor)
    (else
      (Default|LifeLost _aspig_char))))

(event Custom|RandomiseSize
  (Transformation|SetRelativeScale3D (Variables|Default|GetCube) (Math|Conversions|ToVector(Float) (Math|Random|RandomFloatinRange (Variables|Default|GetMinSize) (Variables|Default|GetMaxSize))))
  (switch int (Math|Random|RandomIntegerinRange 0 1)
    (:0
      (Rendering|Material|CreateDynamicMaterialInstance (Variables|Default|GetCube) 0 "/Game/Assets/Obsticles/Tree_mat.Tree_mat" :!class /Script/Engine.PrimitiveComponent))
    (:1
      (Rendering|Material|CreateDynamicMaterialInstance (Variables|Default|GetCube) 0 "/Game/Assets/Obsticles/Tree_2_mat.Tree_2_mat" :!class /Script/Engine.PrimitiveComponent))))

(event EventBeginPlay)

(event EventTick
  (params (DeltaSeconds :type Float%20%28single-precision%29)))

(fn ConstructionScript
  (CallFunction|RandomiseSize))
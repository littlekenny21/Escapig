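; BP_Grass-Corner-L is a corner piece, by its name a grass left turn, that governs turning and wall crashes for PigChar.
; Overlapping TurnZone sets the character's CanTurn flag, and leaving clears it.
; Hits on Wall or Wall2 call LifeLost only when the hit normal nearly matches the character's forward vector, using a dot product check to single out head-on impacts.
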(event OnComponentBeginOverlap(TurnZone)
  (params (OtherActor :type Actor%20Object%20Reference) (OtherComp :type Primitive%20Component%20Object%20Reference) (OtherBodyIndex :type Integer) (bFromSweep :type Boolean) (SweepResult :type Hit%20Result%20Structure%20%28by%20ref%29))
  (bind _aspig_char (Utilities|Casting|CastToPigChar OtherActor))
  (Variables|/Game/Blueprints/Blueprints/PigChar.PigChar_C|SetCanTurn _aspig_char true))

(event OnComponentHit(wall)
  (params (OtherActor :type Actor%20Object%20Reference) (OtherComp :type Primitive%20Component%20Object%20Reference) (NormalImpulse :type Vector :default "0, 0, 0") (Hit :type Hit%20Result%20Structure%20%28by%20ref%29))
  ;[1 1 1] wall Collisions
  (bind _aspig_char (Utilities|Casting|CastToPigChar OtherActor))
  (if (Math|Float|NearlyEqual(Float) (Math|Vector|DotProduct (.normal Hit) (Transformation|GetActorForwardVector _aspig_char)) 1.0 0.01)
    (Default|LifeLost _aspig_char)))

(event OnComponentHit(wall2)
  (params (OtherActor :type Actor%20Object%20Reference) (OtherComp :type Primitive%20Component%20Object%20Reference) (NormalImpulse :type Vector :default "0, 0, 0") (Hit :type Hit%20Result%20Structure%20%28by%20ref%29))
  ;[1 1 1] wall Collisions
  (bind _aspig_char (Utilities|Casting|CastToPigChar OtherActor))
  (if (Math|Float|NearlyEqual(Float) (Math|Vector|DotProduct (.normal Hit) (Transformation|GetActorForwardVector _aspig_char)) 1.0 0.01)
    (Default|LifeLost _aspig_char)))

(event OnComponentEndOverlap(TurnZone)
  (params (OtherActor :type Actor%20Object%20Reference) (OtherComp :type Primitive%20Component%20Object%20Reference) (OtherBodyIndex :type Integer))
  (bind _aspig_char (Utilities|Casting|CastToPigChar OtherActor))
  (Variables|/Game/Blueprints/Blueprints/PigChar.PigChar_C|SetCanTurn _aspig_char false))

(event EventBeginPlay)

(event EventActorBeginOverlap
  (params (OtherActor :type Actor%20Object%20Reference)))

(event EventTick
  (params (DeltaSeconds :type Float%20%28single-precision%29)))

(fn ConstructionScript)
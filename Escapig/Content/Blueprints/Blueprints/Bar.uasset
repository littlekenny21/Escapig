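; Bar actor that slides its Target component back and forth along its local Y axis.
; BeginPlay starts an endless short-Delay loop that steps TargetLoc between -50 and 50, flips TargetDir at either end, and sets the relative location to ten times that value.
; The Target overlap event is empty, and the Accelerate_Box cast and Isboxhitting speed-message logic are disconnected, so they never run.
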(event OnComponentBeginOverlap(Target)
  (params (OtherActor :type Actor%20Object%20Reference) (OtherComp :type Primitive%20Component%20Object%20Reference) (OtherBodyIndex :type Integer) (bFromSweep :type Boolean) (SweepResult :type Hit%20Result%20Structure%20%28by%20ref%29)))

(event EventBeginPlay
  (Utilities|FlowControl|Delay 0.001 :!label _label)
  (Utilities|FlowControl|Sequence
    (:then_0
      (if (== (Variables|Default|GetTargetLoc) 50)
        (Variables|Default|SetTargetDir 0)
        (elif (== (Variables|Default|GetTargetLoc) -50)
          (Variables|Default|SetTargetDir 1)))
      (switch int (Variables|Default|GetTargetDir)
        (:0
          (Math|Integer|DecrementInt (Variables|Default|GetTargetLoc)
            (:%20%20
              _)))
        (:1
          (Math|Integer|IncrementInt (Variables|Default|GetTargetLoc)
            (:%20%20
              _))))
      (Transformation|SetRelativeLocation (Variables|Default|GetTarget) (Math|Vector|MakeVector 0.0 (Math|Conversions|ToFloat(Integer) (* (Variables|Default|GetTargetLoc) 10)) 0.0) false false))
    (:then_1
      (goto _label))))

(fn ConstructionScript)
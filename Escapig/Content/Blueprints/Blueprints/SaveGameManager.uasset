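; Save manager actor that persists selected skin, truffles, unlocked skins and high scores through a GameSave object in one slot.
; BeginPlay loads each field into cached variables, writing a default save if none exists.
; Each save event loads or creates the save, writes its field and reloads that field, except SaveHighScores, which reloads unlocked skins instead.
; NUKE resets cached values and deletes the slot.
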(event Custom|SaveSelectedSkin
  (params (SelectedSkin :type Integer))
  ;[1 1 1] Save which skin is selected
  (bind _returnvalue (SaveGame|DoesSaveGameExist "Jim"))
  (if _returnvalue
    (bind _returnvalue_2 (SaveGame|LoadGamefromSlot "Jim"))
    (Variables|Default|SetSaveSssss _returnvalue_2)
    (bind _asgame_save (Utilities|Casting|CastToGameSave (Variables|Default|GetSaveSssss)))
    (Variables|/Game/Blueprints/Blueprints/GameSave.GameSave_C|SetSelected%20skin _asgame_save SelectedSkin)
    (SaveGame|SaveGametoSlot (Variables|Default|GetSaveSssss) "Jim")
    (else
      (bind _returnvalue_3 (SaveGame|CreateSaveGameObject "/Game/Blueprints/Blueprints/GameSave.GameSave_C"))
      (Variables|Default|SetSaveSssss _returnvalue_3)
      (bind _asgame_save_2 (Utilities|Casting|CastToGameSave (Variables|Default|GetSaveSssss)))
      (Variables|/Game/Blueprints/Blueprints/GameSave.GameSave_C|SetSelected%20skin _asgame_save_2 SelectedSkin)
      (SaveGame|SaveGametoSlot (Variables|Default|GetSaveSssss) "Jim")))
  (CallFunction|LoadSelectedSkinPosition))

(event Custom|SaveTruffles
  (params (Truffles :type Integer))
  ;[1 1 1] Save the number of truffles
  (bind _returnvalue (SaveGame|DoesSaveGameExist "Jim"))
  (if _returnvalue
    (bind _returnvalue_2 (SaveGame|LoadGamefromSlot "Jim"))
    (Variables|Default|SetSaveSssss _returnvalue_2)
    (bind _asgame_save (Utilities|Casting|CastToGameSave (Variables|Default|GetSaveSssss)))
    (Variables|/Game/Blueprints/Blueprints/GameSave.GameSave_C|SetTruffles _asgame_save Truffles)
    (SaveGame|SaveGametoSlot (Variables|Default|GetSaveSssss) "Jim")
    (else
      (bind _returnvalue_3 (SaveGame|CreateSaveGameObject "/Game/Blueprints/Blueprints/GameSave.GameSave_C"))
      (Variables|Default|SetSaveSssss _returnvalue_3)
      (bind _asgame_save_2 (Utilities|Casting|CastToGameSave (Variables|Default|GetSaveSssss)))
      (Variables|/Game/Blueprints/Blueprints/GameSave.GameSave_C|SetTruffles _asgame_save_2 Truffles)
      (SaveGame|SaveGametoSlot (Variables|Default|GetSaveSssss) "Jim")))
  (CallFunction|LoadTruffles))

(event Custom|SaveUnlockedSkins
  (params (UnlockedSkins :type Array%20of%20Booleans))
  ;[1 1 1] Save which skins have been unlocked
  (bind _returnvalue (SaveGame|DoesSaveGameExist "Jim"))
  (if _returnvalue
    (bind _returnvalue_2 (SaveGame|LoadGamefromSlot "Jim"))
    (Variables|Default|SetSaveSssss _returnvalue_2)
    (bind _asgame_save (Utilities|Casting|CastToGameSave (Variables|Default|GetSaveSssss)))
    (Variables|/Game/Blueprints/Blueprints/GameSave.GameSave_C|SetUnlockedSkins _asgame_save UnlockedSkins)
    (SaveGame|SaveGametoSlot (Variables|Default|GetSaveSssss) "Jim")
    (else
      (bind _returnvalue_3 (SaveGame|CreateSaveGameObject "/Game/Blueprints/Blueprints/GameSave.GameSave_C"))
      (Variables|Default|SetSaveSssss _returnvalue_3)
      (bind _asgame_save_2 (Utilities|Casting|CastToGameSave (Variables|Default|GetSaveSssss)))
      (Variables|/Game/Blueprints/Blueprints/GameSave.GameSave_C|SetUnlockedSkins _asgame_save_2 UnlockedSkins)
      (SaveGame|SaveGametoSlot (Variables|Default|GetSaveSssss) "Jim")))
  (CallFunction|LoadUnlockedSkins))

(event Custom|LoadSelectedSkinPosition
  ;[1 1 1] Load selected skin array position from save file
  (bind _returnvalue (SaveGame|DoesSaveGameExist "Jim"))
  (if _returnvalue
    (bind _returnvalue_2 (SaveGame|LoadGamefromSlot "Jim"))
    (Variables|Default|SetSaveSssss _returnvalue_2)
    (bind _asgame_save (Utilities|Casting|CastToGameSave (Variables|Default|GetSaveSssss)))
    (Variables|Default|SetS_SelectedSkin (Variables|/Game/Blueprints/Blueprints/GameSave.GameSave_C|GetSelected%20skin _asgame_save))
    (else
      (CallFunction|NoSaveFile))))

(event Custom|NUKE
  (Development|PrintString "boom")
  (Variables|Default|SetS_HighScore (Variables|Default|Getnoughtarray_HS))
  (Variables|Default|SetS_SelectedSkin 0)
  (Variables|Default|SetS_Truffles 0)
  (Variables|Default|SetS_UnlockedSkins (Variables|Default|Getnoughtarray_US))
  (bind _asgame_save (Utilities|Casting|CastToGameSave (Variables|Default|GetSaveSssss))
    (:then
      (Variables|/Game/Blueprints/Blueprints/GameSave.GameSave_C|SetHighScore _asgame_save (Variables|Default|Getnoughtarray_HS))
      (Variables|/Game/Blueprints/Blueprints/GameSave.GameSave_C|SetTruffles _asgame_save 0)
      (Variables|/Game/Blueprints/Blueprints/GameSave.GameSave_C|SetSelected%20skin _asgame_save 0)
      (Variables|/Game/Blueprints/Blueprints/GameSave.GameSave_C|SetUnlockedSkins _asgame_save (Variables|Default|Getnoughtarray_US))
      (bind _returnvalue (SaveGame|DoesSaveGameExist "jim"))
      (if _returnvalue
        (SaveGame|DeleteGameinSlot "jim")))
    (:CastFailed
      (Development|PrintString "GRR"))))

(event Custom|LoadTruffles
  ;[1 1 1] Load Truffles
  (bind _returnvalue (SaveGame|DoesSaveGameExist "Jim"))
  (if _returnvalue
    (bind _returnvalue_2 (SaveGame|LoadGamefromSlot "Jim"))
    (Variables|Default|SetSaveSssss _returnvalue_2)
    (bind _asgame_save (Utilities|Casting|CastToGameSave (Variables|Default|GetSaveSssss)))
    (Variables|Default|SetS_Truffles (Variables|/Game/Blueprints/Blueprints/GameSave.GameSave_C|GetTruffles _asgame_save))
    (else
      (CallFunction|NoSaveFile))))

(event Custom|NoSaveFile
  ;[1 1 1] If no save file exists, create one with the default values
  (bind _returnvalue (SaveGame|CreateSaveGameObject "/Game/Blueprints/Blueprints/GameSave.GameSave_C"))
  (Variables|Default|SetSaveSssss _returnvalue)
  (Utilities|Casting|CastToGameSave (Variables|Default|GetSaveSssss))
  (SaveGame|SaveGametoSlot (Variables|Default|GetSaveSssss) "Jim"))

(event Custom|LoadUnlockedSkins
  ;[1 1 1] Load Unlocked Skins
  (bind _returnvalue (SaveGame|DoesSaveGameExist "Jim"))
  (if _returnvalue
    (bind _returnvalue_2 (SaveGame|LoadGamefromSlot "Jim"))
    (Variables|Default|SetSaveSssss _returnvalue_2)
    (bind _asgame_save (Utilities|Casting|CastToGameSave (Variables|Default|GetSaveSssss)))
    (Variables|Default|SetS_UnlockedSkins (Variables|/Game/Blueprints/Blueprints/GameSave.GameSave_C|GetUnlockedSkins _asgame_save))
    (else
      (CallFunction|NoSaveFile))))

(event Custom|LoadHighScores
  ;[1 1 1] Load High Scores
  (bind _returnvalue (SaveGame|DoesSaveGameExist "Jim"))
  (if _returnvalue
    (bind _returnvalue_2 (SaveGame|LoadGamefromSlot "Jim"))
    (Variables|Default|SetSaveSssss _returnvalue_2)
    (bind _asgame_save (Utilities|Casting|CastToGameSave (Variables|Default|GetSaveSssss)))
    (Variables|Default|SetS_HighScore (Variables|/Game/Blueprints/Blueprints/GameSave.GameSave_C|GetHighScore _asgame_save))
    (else
      (CallFunction|NoSaveFile))))

(event Custom|SaveHighScores
  (params (HighScores :type Array%20of%20Integers))
  ;[1 1 1] Save the high scores
  (Development|PrintString "Seek and destroy")
  (bind _returnvalue (SaveGame|DoesSaveGameExist "Jim"))
  (if _returnvalue
    (bind _returnvalue_2 (SaveGame|LoadGamefromSlot "Jim"))
    (Variables|Default|SetSaveSssss _returnvalue_2)
    (bind _asgame_save (Utilities|Casting|CastToGameSave (Variables|Default|GetSaveSssss)))
    (Variables|/Game/Blueprints/Blueprints/GameSave.GameSave_C|SetHighScore _asgame_save HighScores)
    (SaveGame|SaveGametoSlot (Variables|Default|GetSaveSssss) "Jim")
    (else
      (bind _returnvalue_3 (SaveGame|CreateSaveGameObject "/Game/Blueprints/Blueprints/GameSave.GameSave_C"))
      (Variables|Default|SetSaveSssss _returnvalue_3)
      (bind _asgame_save_2 (Utilities|Casting|CastToGameSave (Variables|Default|GetSaveSssss)))
      (Variables|/Game/Blueprints/Blueprints/GameSave.GameSave_C|SetHighScore _asgame_save_2 HighScores)
      (SaveGame|SaveGametoSlot (Variables|Default|GetSaveSssss) "Jim")))
  (CallFunction|LoadUnlockedSkins))

(event EventBeginPlay
  (CallFunction|LoadSelectedSkinPosition)
  (CallFunction|LoadTruffles)
  (CallFunction|LoadUnlockedSkins)
  (CallFunction|LoadHighScores))

(event EventActorBeginOverlap
  (params (OtherActor :type Actor%20Object%20Reference)))

(event EventTick
  (params (DeltaSeconds :type Float%20%28single-precision%29)))

(fn ConstructionScript)
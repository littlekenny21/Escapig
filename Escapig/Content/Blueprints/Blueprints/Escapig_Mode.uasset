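; Game mode for a tile-based escape runner that builds the track, shows the run HUD and spawns a Harvester after a short delay.
; BeginPlay lays ten starting tiles when Playing, otherwise it sets the mini-game pawn class.
; AddFloorTile chains random zone-specific tiles by attach transform, recording midpoints in HarvesterPath.
; After a random straight run it inserts a corner, always from the village set because that switch is fixed at zero.
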(event EventBeginPlay
  (Utilities|FlowControl|Delay 0.2)
  (if (Variables|Default|GetPlaying?)
    (bind _returnvalue (UserInterface|CreateWidget "/Game/UMG/RunHud.RunHud_C"))
    (UserInterface|Viewport|AddtoViewport _returnvalue 0)
    (Utilities|FlowControl|Sequence
      (:then_0
        (for _index (range 0 9)
          (CallFunction|AddFloorTile)))
      (:then_1
        (Utilities|FlowControl|Delay 1.0)
        (CallFunction|AddHarvester)))
    (else
      (Variables|Default|SetDefaultPawnClass "/Game/Blueprints/Blueprints/Mini_Game_Pawn.Mini_Game_Pawn_C"))))

(fn ConstructionScript)

(fn AddFloorTile
  (bind _floortiles (Variables|Default|GetFloorTiles))
  (bind _forestfloortiles (Variables|Default|GetForestFloorTiles))
  (bind _villagefloortiles_0 (Variables|Default|GetVillageFloorTiles_0))
  (if (> (Variables|Default|GetCurrent_Straits) (Math|Random|RandomIntegerinRange 5 12))
    (CallFunction|AddCorner)
    (else
      (switch int (Variables|Default|GetZone)
        (:Default
          (bind _returnvalue (Game|SpawnActorfromClass (Utilities|Array|Get(acopy) _villagefloortiles_0 (Math|Random|RandomIntegerinRange 0 (Utilities|Array|LastIndex _villagefloortiles_0))) (Variables|Default|GetNextSpawnPoint) "Undefined" 0 0 :!label _label))
          (bind _asvillage_tile (Utilities|Casting|CastToVillageTile _returnvalue))
          (Variables|/Game/Blueprints/Blueprints/VillageTIle.VillageTile_C|SetID _asvillage_tile (Variables|Default|GetCurrent_Straits))
          (bind _attachtransform (Default|GetAttachTransform _asvillage_tile))
          (Variables|Default|SetNextSpawnPoint _attachtransform)
          (bind _midpoint (Default|GetMidPoint _asvillage_tile))
          (Utilities|Array|Add (Variables|Default|GetHarvesterPath) _midpoint)
          (Variables|Default|SetCurrent_Straits (+ (Variables|Default|GetCurrent_Straits) 1)))
        (:0
          (goto _label))
        (:1
          (bind _returnvalue_2 (Game|SpawnActorfromClass (Utilities|Array|Get(acopy) _floortiles (Math|Random|RandomIntegerinRange 0 (Utilities|Array|LastIndex _floortiles))) (Variables|Default|GetNextSpawnPoint) "Undefined" 0 0))
          (bind _asbp_floor__tile (Utilities|Casting|CastToBP_Floor-Tile _returnvalue_2))
          (Variables|/Game/Blueprints/Blueprints/BP_Floor-Tile.BP_Floor-Tile_C|SetID _asbp_floor__tile (Variables|Default|GetCurrent_Straits))
          (bind _attachtransform_2 (Default|GetAttachTransform _asbp_floor__tile))
          (Variables|Default|SetNextSpawnPoint _attachtransform_2)
          (bind _midpoint_2 (Default|GetMidPoint _asbp_floor__tile))
          (Utilities|Array|Add (Variables|Default|GetHarvesterPath) _midpoint_2)
          (Variables|Default|SetCurrent_Straits (+ (Variables|Default|GetCurrent_Straits) 1)))
        (:2
          (bind _returnvalue_3 (Game|SpawnActorfromClass (Utilities|Array|Get(acopy) _forestfloortiles (Math|Random|RandomIntegerinRange 0 (Utilities|Array|LastIndex _forestfloortiles))) (Variables|Default|GetNextSpawnPoint) "Undefined" 0 0))
          (bind _asvillage_tile_2 (Utilities|Casting|CastToVillageTile _returnvalue_3))
          (Variables|/Game/Blueprints/Blueprints/VillageTIle.VillageTile_C|SetID _asvillage_tile_2 (Variables|Default|GetCurrent_Straits))
          (bind _attachtransform_3 (Default|GetAttachTransform _asvillage_tile_2))
          (Variables|Default|SetNextSpawnPoint _attachtransform_3)
          (bind _midpoint_3 (Default|GetMidPoint _asvillage_tile_2))
          (Utilities|Array|Add (Variables|Default|GetHarvesterPath) _midpoint_3)
          (Variables|Default|SetCurrent_Straits (+ (Variables|Default|GetCurrent_Straits) 1)))))))

(fn AddCorner
  (bind _forestfloorcorners (Variables|Default|GetForestFloorCorners))
  (bind _villagefloor_corners_0 (Variables|Default|GetVillageFloor_Corners_0))
  (bind _floor_corners (Variables|Default|GetFloor_Corners))
  (switch int 0
    (:Default
      (bind _returnvalue (Game|SpawnActorfromClass (Utilities|Array|Get(acopy) _villagefloor_corners_0 (Math|Random|RandomIntegerinRange 0 (Utilities|Array|LastIndex _villagefloor_corners_0))) (Variables|Default|GetNextSpawnPoint) "Undefined" 0 0 :!label _label))
      (bind _asvillage_tile (Utilities|Casting|CastToVillageTile _returnvalue))
      (Variables|/Game/Blueprints/Blueprints/VillageTIle.VillageTile_C|SetID _asvillage_tile (Variables|Default|GetCurrent_Straits))
      (bind _attachtransform (Default|GetAttachTransform _asvillage_tile))
      (Variables|Default|SetNextSpawnPoint _attachtransform)
      (bind _midpoint (Default|GetMidPoint _asvillage_tile))
      (Utilities|Array|Add (Variables|Default|GetHarvesterPath) _midpoint)
      (Variables|Default|SetCurrent_Straits 0))
    (:0
      (goto _label))
    (:1
      (bind _returnvalue_2 (Game|SpawnActorfromClass (Utilities|Array|Get(acopy) _floor_corners (Math|Random|RandomIntegerinRange 0 (Utilities|Array|LastIndex _floor_corners))) (Variables|Default|GetNextSpawnPoint) "Undefined" 0 0))
      (bind _asbp_floor__tile (Utilities|Casting|CastToBP_Floor-Tile _returnvalue_2))
      (Variables|/Game/Blueprints/Blueprints/BP_Floor-Tile.BP_Floor-Tile_C|SetID _asbp_floor__tile (Variables|Default|GetCurrent_Straits))
      (bind _attachtransform_2 (Default|GetAttachTransform _asbp_floor__tile))
      (Variables|Default|SetNextSpawnPoint _attachtransform_2)
      (bind _midpoint_2 (Default|GetMidPoint _asbp_floor__tile))
      (Utilities|Array|Add (Variables|Default|GetHarvesterPath) _midpoint_2)
      (Variables|Default|SetCurrent_Straits 0))
    (:2
      (bind _returnvalue_3 (Game|SpawnActorfromClass (Utilities|Array|Get(acopy) _forestfloorcorners (Math|Random|RandomIntegerinRange 0 (Utilities|Array|LastIndex _forestfloorcorners))) (Variables|Default|GetNextSpawnPoint) "Undefined" 0 0))
      (bind _asvillage_tile_2 (Utilities|Casting|CastToVillageTile _returnvalue_3))
      (Variables|/Game/Blueprints/Blueprints/VillageTIle.VillageTile_C|SetID _asvillage_tile_2 (Variables|Default|GetCurrent_Straits))
      (bind _attachtransform_3 (Default|GetAttachTransform _asvillage_tile_2))
      (Variables|Default|SetNextSpawnPoint _attachtransform_3)
      (bind _midpoint_3 (Default|GetMidPoint _asvillage_tile_2))
      (Utilities|Array|Add (Variables|Default|GetHarvesterPath) _midpoint_3)
      (Variables|Default|SetCurrent_Straits 0))))

(fn AddHarvester
  (Game|SpawnActorfromClass "/Game/Blueprints/Blueprints/Harvester.Harvester_C" (Variables|Default|GetHavesterSpawnPoint) "Undefined" 0 0))
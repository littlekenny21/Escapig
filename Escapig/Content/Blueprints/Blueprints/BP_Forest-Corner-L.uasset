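; Forest left-corner piece for a lane-based runner that manages how the PigChar turns and crashes at the bend.
; Three lane triggers set the pig's lane, turn target location and CanTurn flag.
; TurnZone flags a corner crash on the first PigChar found on entry, then clears turn and crash flags on exit.
; Two walls cost a living pig a life when the hit normal's dot product with its forward vector is nearly one.
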(event OnComponentHit(wall)
  (params (OtherActor :type Actor%20Object%20Reference) (OtherComp :type Primitive%20Component%20Object%20Reference) (NormalImpulse :type Vector :default "0, 0, 0") (Hit :type Hit%20Result%20Structure%20%28by%20ref%29))
  ;[1 1 1] wall Collisions
  (bind _aspig_char (Utilities|Casting|CastToPigChar OtherActor))
  (if (not (Variables|/Game/Blueprints/Blueprints/PigChar.PigChar_C|GetIs_Dead _aspig_char))
    (if (Math|Float|NearlyEqual(Float) (Math|Vector|DotProduct (.normal Hit) (Transformation|GetActorForwardVector _aspig_char)) 1.0 0.01)
      (Default|LifeLost _aspig_char))))

(event OnComponentHit(wall2)
  (params (OtherActor :type Actor%20Object%20Reference) (OtherComp :type Primitive%20Component%20Object%20Reference) (NormalImpulse :type Vector :default "0, 0, 0") (Hit :type Hit%20Result%20Structure%20%28by%20ref%29))
  ;[1 1 1] wall Collisions
  (bind _aspig_char (Utilities|Casting|CastToPigChar OtherActor))
  (if (not (Variables|/Game/Blueprints/Blueprints/PigChar.PigChar_C|GetIs_Dead _aspig_char))
    (if (Math|Float|NearlyEqual(Float) (Math|Vector|DotProduct (.normal Hit) (Transformation|GetActorForwardVector _aspig_char)) 1.0 0.01)
      (Default|LifeLost _aspig_char))))

(event OnComponentEndOverlap(TurnZone)
  (params (OtherActor :type Actor%20Object%20Reference) (OtherComp :type Primitive%20Component%20Object%20Reference) (OtherBodyIndex :type Integer))
  (bind _aspig_char (Utilities|Casting|CastToPigChar OtherActor))
  (Variables|/Game/Blueprints/Blueprints/PigChar.PigChar_C|SetCanTurn _aspig_char false)
  (Variables|/Game/Blueprints/Blueprints/PigChar.PigChar_C|SetCornerCrash _aspig_char false))

(event OnComponentBeginOverlap(TurnZone)
  (params (OtherActor :type Actor%20Object%20Reference) (OtherComp :type Primitive%20Component%20Object%20Reference) (OtherBodyIndex :type Integer) (bFromSweep :type Boolean) (SweepResult :type Hit%20Result%20Structure%20%28by%20ref%29))
  (if (== (Utilities|GetClass OtherActor) "/Game/Blueprints/Blueprints/PigChar.PigChar_C")
    (bind _outactors (Actor|GetAllActorsOfClass "/Game/Blueprints/Blueprints/PigChar.PigChar_C"))
    (Default|OverCornerCashe (Utilities|Array|Get(acopy) _outactors))
    (Variables|/Game/Blueprints/Blueprints/PigChar.PigChar_C|SetCornerCrash (Utilities|Array|Get(acopy) _outactors) true)))

(event OnComponentBeginOverlap(Lane1)
  (params (OtherActor :type Actor%20Object%20Reference) (OtherComp :type Primitive%20Component%20Object%20Reference) (OtherBodyIndex :type Integer) (bFromSweep :type Boolean) (SweepResult :type Hit%20Result%20Structure%20%28by%20ref%29))
  (bind _aspig_char (Utilities|Casting|CastToPigChar OtherActor))
  (Variables|/Game/Blueprints/Blueprints/PigChar.PigChar_C|SetCornerTurnTargetLoc _aspig_char (Transformation|GetWorldLocation (Variables|Default|GetLane1Target)))
  (Variables|/Game/Blueprints/Blueprints/PigChar.PigChar_C|SetCanTurn _aspig_char true)
  (Variables|/Game/Blueprints/Blueprints/PigChar.PigChar_C|SetLane _aspig_char 1))

(event OnComponentBeginOverlap(Lane2)
  (params (OtherActor :type Actor%20Object%20Reference) (OtherComp :type Primitive%20Component%20Object%20Reference) (OtherBodyIndex :type Integer) (bFromSweep :type Boolean) (SweepResult :type Hit%20Result%20Structure%20%28by%20ref%29))
  (bind _aspig_char (Utilities|Casting|CastToPigChar OtherActor))
  (Variables|/Game/Blueprints/Blueprints/PigChar.PigChar_C|SetCornerTurnTargetLoc _aspig_char (Transformation|GetWorldLocation (Variables|Default|GetLane2Target)))
  (Variables|/Game/Blueprints/Blueprints/PigChar.PigChar_C|SetCanTurn _aspig_char true)
  (Variables|/Game/Blueprints/Blueprints/PigChar.PigChar_C|SetLane _aspig_char 2))

(event OnComponentBeginOverlap(Lane3)
  (params (OtherActor :type Actor%20Object%20Reference) (OtherComp :type Primitive%20Component%20Object%20Reference) (OtherBodyIndex :type Integer) (bFromSweep :type Boolean) (SweepResult :type Hit%20Result%20Structure%20%28by%20ref%29))
  (bind _aspig_char (Utilities|Casting|CastToPigChar OtherActor))
  (Variables|/Game/Blueprints/Blueprints/PigChar.PigChar_C|SetCornerTurnTargetLoc _aspig_char (Transformation|GetWorldLocation (Variables|Default|GetLane3Target)))
  (Variables|/Game/Blueprints/Blueprints/PigChar.PigChar_C|SetCanTurn _aspig_char true)
  (Variables|/Game/Blueprints/Blueprints/PigChar.PigChar_C|SetLane _aspig_char 3))

(fn ConstructionScript)
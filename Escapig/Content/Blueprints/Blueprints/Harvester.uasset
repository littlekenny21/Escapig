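; Harvester that chases the pig, following Escapig_Mode's HarvesterPath waypoints, or fixed-axis targets in minigame mode.
; Tick steps it toward each destination, with HarvesterSpeed as a divisor, so it rubber-bands faster when the pig is distant.
; Overlapping the pig halts it and costs a life once until reset, while PigStopped knocks it back before resuming.
; SlowHarvester temporarily halves HarvesterSpeed, though Tick overwrites that outside minigames.
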(event Custom|PigStopped
  (bind _returnvalue (Transformation|GetActorRotation))
  (bind _returnvalue_2 (Transformation|GetActorLocation))
  (bind _yaw (Math|Rotator|BreakRotator _returnvalue))
  ;[1 1 1] Move Back
  (Variables|Default|SetHitPig true)
  (Utilities|FlowControl|Delay 0.1)
  (if (Math|Float|NearlyEqual(Float) _yaw 0.0 0.1)
    (Transformation|SetActorLocation (+ _returnvalue_2 "-500.000000,0.000000, 0") false false)
    (elif (Math|Float|NearlyEqual(Float) _yaw 9e+01 0.1)
      (Transformation|SetActorLocation (+ _returnvalue_2 "0.000000,-500.000000, 0") false false)
      (elif (Math|Float|NearlyEqual(Float) _yaw -9e+01 0.1)
        (Transformation|SetActorLocation (+ _returnvalue_2 "0.000000,500.000000, 0") false false)
        (else
          (Transformation|SetActorLocation (+ _returnvalue_2 "500.000000,0.000000, 0") false false)))))
  (Utilities|FlowControl|Delay 1.5)
  (CallFunction|ResetHitPig)
  (Variables|Default|SetStartPosition (Transformation|GetActorLocation)))

(event Custom|Slow%20Harvester
  ;[1 1 1] Method to be called by the Slow Harvester pickup to slow the harvester down
  (Variables|Default|SetHarvesterSpeed (/ (Variables|Default|GetHarvesterSpeed) 2.0))
  (Utilities|FlowControl|Delay 6.0)
  (Variables|Default|SetHarvesterSpeed (Variables|Default|GetHarvesterDefaultSpeed)))

(event Custom|GetNextDestination
  (bind _returnvalue (Transformation|GetActorLocation))
  ;[1 1 1] Get Next Destination
  (if (Variables|Default|GetMini_Game)
    (Variables|Default|SetHarvesterSpeed 8e+01)
    (if (Variables|Default|GetMince)
      (bind _output_get (Variables|Default|SetStartPosition (Transformation|GetActorLocation)))
      (Variables|Default|SetDestination (Math|Vector|MakeVector (.X (Math|Vector|BreakVector _output_get)) 1e+03 (.Z (Math|Vector|BreakVector _output_get))))
      (else
        (bind _output_get_2 (Variables|Default|SetStartPosition (Transformation|GetActorLocation)))
        (Variables|Default|SetDestination (Math|Vector|MakeVector (+ (.X (Math|Vector|BreakVector _output_get_2)) 1e+02) (.Y (Math|Vector|BreakVector _output_get_2)) (.Z (Math|Vector|BreakVector _output_get_2))))))
    (else
      (bind _asescapig_mode (Utilities|Casting|CastToEscapig_Mode (Game|GetGameMode)))
      (Variables|Default|SetDestination (Math|Vector|MakeVector (.X (Math|Vector|BreakVector (Utilities|Array|Get(acopy) (Variables|/Game/Blueprints/Blueprints/Escapig_Mode.Escapig_Mode_C|GetHarvesterPath _asescapig_mode)))) (.Y (Math|Vector|BreakVector (Utilities|Array|Get(acopy) (Variables|/Game/Blueprints/Blueprints/Escapig_Mode.Escapig_Mode_C|GetHarvesterPath _asescapig_mode)))) (.Z (Math|Vector|BreakVector _returnvalue))))
      (Utilities|Array|RemoveIndex (Variables|/Game/Blueprints/Blueprints/Escapig_Mode.Escapig_Mode_C|GetHarvesterPath _asescapig_mode))
      (bind _output_get_3 (Variables|Default|SetStartPosition _returnvalue))
      (if (Math|Float|NearlyEqual(Float) (- (.Y (Math|Vector|BreakVector (Variables|Default|GetDestination))) (.Y (Math|Vector|BreakVector _output_get_3))) 0.0 0.1)
        (if (>= (- (.X (Math|Vector|BreakVector (Variables|Default|GetDestination))) (.X (Math|Vector|BreakVector _output_get_3))) 0.0)
          (Transformation|SetActorRotation "0,0.000000, 0")
          (else
            (Transformation|SetActorRotation "0.000000,180.000000, 0")))
        (elif (Math|Float|NearlyEqual(Float) (- (.X (Math|Vector|BreakVector (Variables|Default|GetDestination))) (.X (Math|Vector|BreakVector _output_get_3))) 0.0 0.1)
          (if (>= (- (.Y (Math|Vector|BreakVector (Variables|Default|GetDestination))) (.Y (Math|Vector|BreakVector _output_get_3))) 0.0)
            (Transformation|SetActorRotation "0.000000,90.000000,0.000000")
            (else
              (Transformation|SetActorRotation "0.000000,270.000000, 0"))))))))

(event Custom|ResetHitPig
  ;[1 1 1] Hit the pig
  (Variables|Default|SetHitPig false)
  (Utilities|FlowControl|DoOnce false) ; enters at Reset
)

(event EventBeginPlay
  ;[1 1 1] Set the default speed to be reset to after the harvester iis slowed
  (Variables|Default|SetHarvesterDefaultSpeed (Variables|Default|GetHarvesterSpeed)))

(event EventActorBeginOverlap
  (params (OtherActor :type Actor%20Object%20Reference))
  ;[1 1 1] Hit the pig
  (bind _aspig_char (Utilities|Casting|CastToPigChar OtherActor))
  (Variables|Default|SetHitPig true)
  (Utilities|FlowControl|DoOnce false
    (:Completed
      (Default|LifeLost _aspig_char))))

(event EventTick
  (params (DeltaSeconds :type Float%20%28single-precision%29))
  (bind _returnvalue (Transformation|GetActorLocation))
  (bind _startposition (Variables|Default|GetStartPosition))
  (bind _destination (Variables|Default|GetDestination))
  ;[1 1 1] On Tick
  (if (not (Variables|Default|GetHitPig))
    (if (Variables|Default|GetInitialised)
      (if (Math|Vector|Equal(Vector) _returnvalue _destination 1e+01)
        (CallFunction|GetNextDestination :!label _label)
        (else
          (Transformation|SetActorLocation (+ _returnvalue (* (Class|KismetMathLibrary|GetDirectionVector _startposition _destination) (/ (Math|Vector|VectorLength (- _startposition _destination)) (* 1.75 (Variables|Default|GetHarvesterSpeed))))) false false)
          (if (not (Variables|Default|GetMini_Game))
            (bind _outactors (Actor|GetAllActorsOfClass "/Game/Blueprints/Blueprints/PigChar.PigChar_C"))
            (if (> (Math|Vector|VectorLength (- (Transformation|GetActorLocation) (Transformation|GetActorLocation (Utilities|Array|Get(acopy) _outactors)))) 6e+02)
              (Variables|Default|SetHarvesterSpeed 15.0)
              (else
                (Variables|Default|SetHarvesterSpeed 35.0))))))
      (else
        (Utilities|FlowControl|Sequence
          (:then_0
            (goto _label))
          (:then_1
            (Variables|Default|SetInitialised true)))))))

(fn ConstructionScript)